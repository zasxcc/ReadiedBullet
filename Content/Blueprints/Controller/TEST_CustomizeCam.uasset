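; Test Blueprint for a customization camera, judging by its name, that orbits and zooms through keyboard and mouse input.
; W, A, S and D turn the spring arm in 90-degree world-rotation steps and store its target rotation in CamRot, which nothing here reads.
; The mouse wheel nudges the camera along its relative X axis.
; BeginPlay shows the cursor, and Tick prints the arm's target rotation for debugging.
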(event EventBeginPlay
  (Variables|/Script/Engine.PlayerController|SetbShowMouseCursor (Game|GetPlayerController 0) true)
  (Variables|Default|SetCamRot "0, 0, 0"))

(event Collision|EventActorBeginOverlap
  (params (OtherActor :type Actor%20Object%20Reference)))

(event EventTick
  (params (DeltaSeconds :type Float%20%28single-precision%29))
  (Development|PrintString (Utilities|String|ToString(Rotator) (Class|SpringArmComponent|GetTargetRotation (Variables|Default|GetSrpin))) true true "(R=0.000000,G=0.660000,B=1.000000,A=1.000000)" 0.0))

(event Input|MouseEvents|MouseWheelUp
  (params (Key :type Key%20Structure))
  (:Pressed
    (Transformation|AddRelativeLocation (Variables|Default|GetCamera) "10.000000, 0, 0" false false)))

(event Input|KeyboardEvents|A
  (params (Key :type Key%20Structure))
  (:Pressed
    (Transformation|AddWorldRotation (Variables|Default|GetSrpin) "0.000000, 0,-90.000000" false false)
    (Variables|Default|SetCamRot (Class|SpringArmComponent|GetTargetRotation (Variables|Default|GetSrpin)))))

(event Input|KeyboardEvents|D
  (params (Key :type Key%20Structure))
  (:Pressed
    (Transformation|AddWorldRotation (Variables|Default|GetSrpin) "0.000000, 0,90.000000" false false)
    (Variables|Default|SetCamRot (Class|SpringArmComponent|GetTargetRotation (Variables|Default|GetSrpin)))))

(event Input|KeyboardEvents|W
  (params (Key :type Key%20Structure))
  (:Pressed
    (Transformation|AddWorldRotation (Variables|Default|GetSrpin) "-90.000000, 0,0.000000" false false)
    (Variables|Default|SetCamRot (Class|SpringArmComponent|GetTargetRotation (Variables|Default|GetSrpin)))))

(event Input|KeyboardEvents|S
  (params (Key :type Key%20Structure))
  (:Pressed
    (Transformation|AddWorldRotation (Variables|Default|GetSrpin) "90.000000, 0,0.000000" false false)
    (Variables|Default|SetCamRot (Class|SpringArmComponent|GetTargetRotation (Variables|Default|GetSrpin)))))

(event Input|MouseEvents|MouseWheelDown
  (params (Key :type Key%20Structure))
  (:Pressed
    (Transformation|AddRelativeLocation (Variables|Default|GetCamera) "-10.000000, 0, 0" false false)))

(fn ConstructionScript)