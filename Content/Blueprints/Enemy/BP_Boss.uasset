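; BP_Boss is an enemy boss that engages once the player comes within a fixed distance.
; Tick polls that distance, then latches an attack flag and reveals the HP bar hidden at BeginPlay.
; While attacking, the mesh turns to face the player each tick, with a yaw offset.
; On actor overlap it destroys itself if MaxHP is near zero; the collision-disabling nodes never run.
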(event EventBeginPlay
  (Rendering|SetVisibility (Variables|Default|GetHPBarWidget) false false))

(event Collision|EventActorBeginOverlap
  (params (OtherActor :type Actor%20Object%20Reference))
  (if (< (Variables|Default|GetMaxHP) 0.001)
    (Actor|DestroyActor)))

(event EventTick
  (params (DeltaSeconds :type Float%20%28single-precision%29))
  (bind _mesh (Variables|Character|GetMesh))
  (if (Variables|Default|GetbIsAttack)
    (Transformation|SetWorldRotation _mesh (Math|Rotator|FindLookatRotation (Transformation|GetActorLocation) (Transformation|GetActorLocation (Game|Player|GetPlayerPawn 0))) false false)
    (Transformation|AddWorldRotation _mesh "0,-90.000000, 0" false false)
    (elif (> 6.5e+03 (Math|Vector|Distance(Vector) (Transformation|GetActorLocation) (Transformation|GetActorLocation (Game|GetPlayerCharacter 0))))
      (Variables|Default|SetbIsAttack true)
      (Rendering|SetVisibility (Variables|Default|GetHPBarWidget) true false))))

(fn ConstructionScript)