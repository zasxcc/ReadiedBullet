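; BP_AIBullet is an enemy AI bullet that reacts to the first actor it overlaps and then destroys itself.
; It identifies the player by comparing the actor's entire Tags array to PlayerTag, rather than checking for one tag.
; A match spawns a blood splash slightly above the actor's origin, while any other actor gets a shockwave effect and hit sound there.
; The graph applies no damage.
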(event EventBeginPlay)

(event Collision|EventActorBeginOverlap
  (params (OtherActor :type Actor%20Object%20Reference))
  (bind _returnvalue (Transformation|GetActorLocation OtherActor))
  (bind _returnvalue_2 (+ _returnvalue "0,0.000000,30.000000"))
  (if (Utilities|Array|Identical (Variables|/Script/Engine.Actor|GetTags OtherActor) (Variables|Default|GetPlayerTag))
    (Effects|SpawnEmitteratLocation "/Game/Effects/WeaponEffects/BloodImpact/P_blood_splash_02.P_blood_splash_02" _returnvalue_2)
    (else
      (Effects|SpawnEmitteratLocation "/Game/Effects/FXVarietyPack/Particles/P_ky_shotShockwave.P_ky_shotShockwave" _returnvalue_2 (Transformation|GetActorRotation OtherActor))
      (Audio|PlaySoundatLocation "/Game/Sound/GinHit.GinHit" _returnvalue_2 "0, 0, 0" 1.0 1.0 0.0 "/Game/Sound/SoundAttenuation.SoundAttenuation" 0 0)))
  (Actor|DestroyActor))

(event EventTick
  (params (DeltaSeconds :type Float%20%28single-precision%29)))

(fn ConstructionScript)