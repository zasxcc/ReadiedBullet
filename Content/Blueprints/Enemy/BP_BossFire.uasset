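; BP_BossFire is a boss fire projectile that launches along local Y with a random downward velocity on BeginPlay.
; Any overlap plays two explosion effects and a sound, then destroys the projectile.
; If the overlapped actor's tags exactly match the NewVar1 array it only explodes.
; Otherwise it also spawns one of three random BP_FireAshes variants at the Cube's transform.
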(event EventBeginPlay
  (Game|Components|ProjectileMovement|SetVelocityinLocalSpace (Variables|Default|GetProjectileMovement) (Math|Vector|MakeVector 0.0 1.5e+03 (Math|Random|RandomFloatinRange -3.5e+02 -5.5e+02))))

(event Collision|EventActorBeginOverlap
  (params (OtherActor :type Actor%20Object%20Reference))
  (bind _returnvalue (Transformation|GetActorLocation))
  (bind _returnvalue_2 (Transformation|GetActorLocation))
  (if (Utilities|Array|Identical (Variables|/Script/Engine.Actor|GetTags OtherActor) (Variables|Default|GetNewVar_1))
    (Effects|SpawnEmitteratLocation "/Game/Effects/AdvancedMagicFX13/Particles/P_ky_explosion2.P_ky_explosion2" _returnvalue_2)
    (Effects|SpawnEmitteratLocation "/Game/Effects/InfinityBladeEffects/Effects/FX_Skill_RockBurst/P_RBurst_Fire_Burst_Area_01.P_RBurst_Fire_Burst_Area_01" _returnvalue_2)
    (Audio|PlaySoundatLocation "/Game/Sound/BossFire_Sound.BossFire_Sound" _returnvalue_2 "0, 0, 0" 1.0 1.0 0.0 "/Game/Sound/SoundAttenuation.SoundAttenuation" 0 0)
    (Actor|DestroyActor)
    (else
      (Effects|SpawnEmitteratLocation "/Game/Effects/AdvancedMagicFX13/Particles/P_ky_explosion2.P_ky_explosion2" _returnvalue)
      (Effects|SpawnEmitteratLocation "/Game/Effects/InfinityBladeEffects/Effects/FX_Skill_RockBurst/P_RBurst_Fire_Burst_Area_01.P_RBurst_Fire_Burst_Area_01" _returnvalue)
      (bind _output_get (Variables|Default|SetSpawnTransform (Transformation|GetWorldTransform (Variables|Default|GetCube))))
      (Actor|DestroyActor)
      (bind _output_get_2 (Variables|Default|Setrand (Math|Random|RandomIntegerinRange 0 2)))
      (switch int _output_get_2
        (:0
          (bind _returnvalue_3 (Game|SpawnActorfromClass "/Game/Blueprints/Enemy/BP_Fireashes.BP_FireAshes_C" _output_get "AlwaysSpawn" 0 0))
          (Audio|PlaySoundatLocation "/Game/Sound/BossFire_Sound.BossFire_Sound" (Transformation|GetActorLocation _returnvalue_3) "0, 0, 0" 1.0 1.0 0.0 "/Game/Sound/SoundAttenuation.SoundAttenuation" 0 0))
        (:1
          (bind _returnvalue_4 (Game|SpawnActorfromClass "/Game/Blueprints/Enemy/BP_FireAshes_2.BP_FireAshes_2_C" _output_get "AlwaysSpawn" 0 0))
          (Audio|PlaySoundatLocation "/Game/Sound/BossFire_Sound.BossFire_Sound" (Transformation|GetActorLocation _returnvalue_4) "0, 0, 0" 1.0 1.0 0.0 "/Game/Sound/SoundAttenuation.SoundAttenuation" 0 0))
        (:2
          (bind _returnvalue_5 (Game|SpawnActorfromClass "/Game/Blueprints/Enemy/BP_FireAshes_3.BP_FireAshes_3_C" _output_get "AlwaysSpawn" 0 0))
          (Audio|PlaySoundatLocation "/Game/Sound/BossFire_Sound.BossFire_Sound" (Transformation|GetActorLocation _returnvalue_5) "0, 0, 0" 1.0 1.0 0.0 "/Game/Sound/SoundAttenuation.SoundAttenuation" 0 0))))))

(event EventTick
  (params (DeltaSeconds :type Float%20%28single-precision%29)))

(fn ConstructionScript)