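; BP_GunTower is an enemy gun turret that flips upright and shoots when the player comes within range.
; Tick checks player distance, rolling the actor toward upright when near and back over when far.
; Once upright, the mesh faces the player, and a frame-counted timer periodically plays the gun animation and attenuated sound, then calls Fire, whose body is not defined here.
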(event EventBeginPlay)

(event Collision|EventActorBeginOverlap
  (params (OtherActor :type Actor%20Object%20Reference)))

(event EventTick
  (params (DeltaSeconds :type Float%20%28single-precision%29))
  (if (> 2.5e+03 (Math|Vector|Distance(Vector) (Transformation|GetActorLocation) (Transformation|GetActorLocation (Game|GetPlayerCharacter 0))))
    (if (>= (.roll (Transformation|GetActorRotation)) 5.0)
      (Class|Actor|AddActorWorldRotation "0, 0,-5.000000")
      (else
        (Transformation|SetWorldRotation (Variables|Character|GetMesh) (Math|Rotator|FindLookatRotation (Transformation|GetActorLocation) (Transformation|GetActorLocation (Game|Player|GetPlayerPawn 0))) false false)
        (bind _output_get (Variables|Default|SetFireTime (+ (Variables|Default|GetFireTime) 1.0)))
        (if (> _output_get 4e+01)
          (Components|Animation|PlayAnimation (Variables|Character|GetMesh) "/Game/CSC/Animations/Anim_CSC_Gun4.Anim_CSC_Gun4" false)
          (Audio|PlaySoundatLocation "/Game/Sound/ShockWave.ShockWave" (Transformation|GetWorldLocation (Variables|Character|GetMesh)) "0, 0, 0" 1.0 1.0 0.0 "/Game/Sound/SoundAttenuation.SoundAttenuation" 0 0)
          (Class|GunTower|Fire)
          (Variables|Default|SetFireTime 0.0))))
    (elif (<= (.roll (Transformation|GetActorRotation)) 175.0)
      (Class|Actor|AddActorWorldRotation "0, 0,5.000000"))))

(fn ConstructionScript)