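; Camera Blueprint for a customization screen that shows the actor-spawn widget and moves its camera along local X with the mouse wheel.
; Tick polls RBGameInstance stage-clear flags, then swaps the widget for a preloaded loading screen and opens the Nature or City level.
; SaveCustomCamSlot copies the widget's box, cylinder and sphere transform slots into local variables.
; SaveGameInstanceSlot is empty, noted as converted to C++, leaving its old copy logic disconnected.
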(event EventBeginPlay
  (bind _returnvalue (Game|GetPlayerController 0))
  (bind _returnvalue_2 (UserInterface|CreateWidget "/Game/UI/WBP_NaturLoading.WBP_NaturLoading_C" _returnvalue))
  (Variables|Default|SetNatureLoading _returnvalue_2)
  (bind _returnvalue_3 (UserInterface|CreateWidget "/Game/UI/WBP_CityLoading.WBP_CityLoading_C" _returnvalue))
  (Variables|Default|SetCityloading _returnvalue_3)
  (bind _returnvalue_4 (UserInterface|CreateWidget "/Game/UI/WBP_CustomizeActorSpawn.WBP_CustomizeActorSpawn_C" _returnvalue))
  (bind _output_get (Variables|Default|Setwidget _returnvalue_4))
  (UserInterface|Viewport|AddtoViewport _output_get 0))

(event Collision|EventActorBeginOverlap
  (params (OtherActor :type Actor%20Object%20Reference)))

(event EventTick
  (params (DeltaSeconds :type Float%20%28single-precision%29))
  (bind _asrbgame_instance (Utilities|Casting|CastToRBGameInstance (Game|GetGameInstance)))
  (if (Variables|/Script/ReadiedBullet.RBGameInstance|GetclearStage1 _asrbgame_instance)
    (Variables|/Script/ReadiedBullet.RBGameInstance|SetclearStage1 _asrbgame_instance false)
    (Widget|SetVisibility (Variables|Default|Getwidget) "Collapsed")
    (UserInterface|Viewport|AddtoViewport (Variables|Default|GetNatureLoading) 0)
    (Game|LoadStreamLevel(byName) "Nature" false)
    (Game|OpenLevel(byName) "Nature" false "dsad")
    (elif (Variables|/Script/ReadiedBullet.RBGameInstance|GetclearStage2 _asrbgame_instance)
      (Variables|/Script/ReadiedBullet.RBGameInstance|SetclearStage2 _asrbgame_instance false)
      (Widget|SetVisibility (Variables|Default|Getwidget) "Collapsed")
      (UserInterface|Viewport|AddtoViewport (Variables|Default|GetCityloading) 0)
      (Game|LoadStreamLevel(byName) "City" false)
      (Game|OpenLevel(byName) "City" false))))

(event Input|MouseEvents|MouseWheelDown
  (params (Key :type Key%20Structure))
  (:Pressed
    (Transformation|AddRelativeLocation (Variables|Default|GetCameraComp) "-20.000000, 0, 0" false false)))

(event Input|MouseEvents|MouseWheelUp
  (params (Key :type Key%20Structure))
  (:Pressed
    (Transformation|AddRelativeLocation (Variables|Default|GetCameraComp) "20.000000, 0, 0" false false)))

(fn ConstructionScript)

(fn SaveCustomCamSlot
  (bind _aswbp_customize_actor_spawn (Utilities|Casting|CastToWBP_CustomizeActorSpawn (Variables|Default|Getwidget)))
  (Variables|Default|SetTransformSlotBox1 (Variables|/Game/UI/WBP_CustomizeActorSpawn.WBP_CustomizeActorSpawn_C|GetSaveTransform_Box1 _aswbp_customize_actor_spawn))
  (Variables|Default|SetTransformSlotCylinder1 (Variables|/Game/UI/WBP_CustomizeActorSpawn.WBP_CustomizeActorSpawn_C|GetSaveTransform_Cylinder1 _aswbp_customize_actor_spawn))
  (Variables|Default|SetTransformSlotSphere1 (Variables|/Game/UI/WBP_CustomizeActorSpawn.WBP_CustomizeActorSpawn_C|GetSaveTransform_Sphere1 _aswbp_customize_actor_spawn))
  (Variables|Default|SetTransformSlotBox2 (Variables|/Game/UI/WBP_CustomizeActorSpawn.WBP_CustomizeActorSpawn_C|GetSaveTransform_Box2 _aswbp_customize_actor_spawn))
  (Variables|Default|SetTransformSlotCylinder2 (Variables|/Game/UI/WBP_CustomizeActorSpawn.WBP_CustomizeActorSpawn_C|GetSaveTransform_Cylinder2 _aswbp_customize_actor_spawn))
  (Variables|Default|SetTransformSlotSphere2 (Variables|/Game/UI/WBP_CustomizeActorSpawn.WBP_CustomizeActorSpawn_C|GetSaveTransform_Sphere2 _aswbp_customize_actor_spawn))
  (Variables|Default|SetTransformSlotBox3 (Variables|/Game/UI/WBP_CustomizeActorSpawn.WBP_CustomizeActorSpawn_C|GetSaveTransform_Box3 _aswbp_customize_actor_spawn))
  (Variables|Default|SetTransformSlotCylinder3 (Variables|/Game/UI/WBP_CustomizeActorSpawn.WBP_CustomizeActorSpawn_C|GetSaveTransform_Cylinder3 _aswbp_customize_actor_spawn))
  (Variables|Default|SetTransformSlotSphere3 (Variables|/Game/UI/WBP_CustomizeActorSpawn.WBP_CustomizeActorSpawn_C|GetSaveTransform_Sphere3 _aswbp_customize_actor_spawn)))

(fn SaveGameInstanceSlot
  ;[1 1 1] C++화 완료
)