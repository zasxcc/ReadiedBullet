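; BP_TEST is a test actor for a mouse-draggable piece that snaps onto another actor on release.
; While clicked, Tick moves StaticMesh to the cursor trace's XY at a fixed height.
; Six directional components set per-side overlap flags and a shared Overlap flag.
; On release, each flagged side teleports the root to a child component of OtherActor picked by hard-coded index, so the last matching side wins.
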(event OnComponentBeginOverlap(Left)
  (params (OverlappedComponent :type Primitive%20Component%20Object%20Reference) (OtherActor :type Actor%20Object%20Reference) (OtherComp :type Primitive%20Component%20Object%20Reference) (OtherBodyIndex :type Integer) (bFromSweep :type Boolean) (SweepResult :type Hit%20Result%20Structure%20%28by%20ref%29))
  (Variables|Default|SetbOverlap true)
  (Variables|Default|SetbOverlapLeft true))

(event OnComponentBeginOverlap(Up)
  (params (OverlappedComponent :type Primitive%20Component%20Object%20Reference) (OtherActor :type Actor%20Object%20Reference) (OtherComp :type Primitive%20Component%20Object%20Reference) (OtherBodyIndex :type Integer) (bFromSweep :type Boolean) (SweepResult :type Hit%20Result%20Structure%20%28by%20ref%29))
  (Variables|Default|SetbOverlap true)
  (Variables|Default|SetbOverlapUp true))

(event OnComponentEndOverlap(Up)
  (params (OverlappedComponent :type Primitive%20Component%20Object%20Reference) (OtherActor :type Actor%20Object%20Reference) (OtherComp :type Primitive%20Component%20Object%20Reference) (OtherBodyIndex :type Integer))
  (Variables|Default|SetbOverlap false)
  (Variables|Default|SetbOverlapUp false))

(event OnComponentBeginOverlap(Down)
  (params (OverlappedComponent :type Primitive%20Component%20Object%20Reference) (OtherActor :type Actor%20Object%20Reference) (OtherComp :type Primitive%20Component%20Object%20Reference) (OtherBodyIndex :type Integer) (bFromSweep :type Boolean) (SweepResult :type Hit%20Result%20Structure%20%28by%20ref%29))
  (Variables|Default|SetbOverlap true)
  (Variables|Default|SetbOverlapDown true))

(event OnComponentEndOverlap(Down)
  (params (OverlappedComponent :type Primitive%20Component%20Object%20Reference) (OtherActor :type Actor%20Object%20Reference) (OtherComp :type Primitive%20Component%20Object%20Reference) (OtherBodyIndex :type Integer))
  (Variables|Default|SetbOverlap false)
  (Variables|Default|SetbOverlapDown false))

(event OnComponentBeginOverlap(Front)
  (params (OverlappedComponent :type Primitive%20Component%20Object%20Reference) (OtherActor :type Actor%20Object%20Reference) (OtherComp :type Primitive%20Component%20Object%20Reference) (OtherBodyIndex :type Integer) (bFromSweep :type Boolean) (SweepResult :type Hit%20Result%20Structure%20%28by%20ref%29))
  (Variables|Default|SetbOverlap true)
  (Variables|Default|SetbOverlapFront true))

(event OnComponentEndOverlap(Front)
  (params (OverlappedComponent :type Primitive%20Component%20Object%20Reference) (OtherActor :type Actor%20Object%20Reference) (OtherComp :type Primitive%20Component%20Object%20Reference) (OtherBodyIndex :type Integer))
  (Variables|Default|SetbOverlap false)
  (Variables|Default|SetbOverlapFront false))

(event OnComponentBeginOverlap(Back)
  (params (OverlappedComponent :type Primitive%20Component%20Object%20Reference) (OtherActor :type Actor%20Object%20Reference) (OtherComp :type Primitive%20Component%20Object%20Reference) (OtherBodyIndex :type Integer) (bFromSweep :type Boolean) (SweepResult :type Hit%20Result%20Structure%20%28by%20ref%29))
  (Variables|Default|SetbOverlap true)
  (Variables|Default|SetbOverlapBack true))

(event OnComponentEndOverlap(Back)
  (params (OverlappedComponent :type Primitive%20Component%20Object%20Reference) (OtherActor :type Actor%20Object%20Reference) (OtherComp :type Primitive%20Component%20Object%20Reference) (OtherBodyIndex :type Integer))
  (Variables|Default|SetbOverlap false)
  (Variables|Default|SetbOverlapBack false))

(event OnClicked(StaticMesh)
  (params (TouchedComponent :type Primitive%20Component%20Object%20Reference) (ButtonPressed :type Key%20Structure))
  ;[1 1 1] 마우스 클릭&언클릭
  (Variables|Default|SetbOnCusor true))

(event OnReleased(StaticMesh)
  (params (TouchedComponent :type Primitive%20Component%20Object%20Reference) (ButtonReleased :type Key%20Structure))
  ;[1 1 1] 마우스 클릭&언클릭
  (Variables|Default|SetbOnCusor false)
  (if (Variables|Default|GetbOverlap)
    (Utilities|FlowControl|Sequence
      (:then_0
        (if (Variables|Default|GetbOverlapLeft)
          (Variables|Default|SetVector (Transformation|GetWorldLocation (Components|GetChildComponent (Variables|/Script/Engine.Actor|GetRootComponent (stale OnComponentBeginOverlap(Left) OtherActor)) 1)))
          (Transformation|SetWorldLocation (Variables|Transformation|GetRootComponent) (Variables|Default|GetVector) false false :!label _label)))
      (:then_1
        (if (Variables|Default|GetbOverlapRight)
          (Variables|Default|SetVector (Transformation|GetWorldLocation (Components|GetChildComponent (Variables|/Script/Engine.Actor|GetRootComponent (stale OnComponentBeginOverlap(Right) OtherActor)) 6)))
          (goto _label)))
      (:then_2
        (if (Variables|Default|GetbOverlapUp)
          (Variables|Default|SetVector (Transformation|GetWorldLocation (Components|GetChildComponent (Variables|/Script/Engine.Actor|GetRootComponent (stale OnComponentBeginOverlap(Up) OtherActor)) 5)))
          (goto _label)))
      (:then_3
        (if (Variables|Default|GetbOverlapDown)
          (Variables|Default|SetVector (Transformation|GetWorldLocation (Components|GetChildComponent (Variables|/Script/Engine.Actor|GetRootComponent (stale OnComponentBeginOverlap(Down) OtherActor)) 4)))
          (goto _label)))
      (:then_4
        (if (Variables|Default|GetbOverlapFront)
          (Variables|Default|SetVector (Transformation|GetWorldLocation (Components|GetChildComponent (Variables|/Script/Engine.Actor|GetRootComponent (stale OnComponentBeginOverlap(Front) OtherActor)) 2)))
          (goto _label)))
      (:then_5
        (if (Variables|Default|GetbOverlapBack)
          (Variables|Default|SetVector (Transformation|GetWorldLocation (Components|GetChildComponent (Variables|/Script/Engine.Actor|GetRootComponent (stale OnComponentBeginOverlap(Back) OtherActor)) 3)))
          (goto _label))))))

(event OnComponentEndOverlap(Left)
  (params (OverlappedComponent :type Primitive%20Component%20Object%20Reference) (OtherActor :type Actor%20Object%20Reference) (OtherComp :type Primitive%20Component%20Object%20Reference) (OtherBodyIndex :type Integer))
  (Variables|Default|SetbOverlap false)
  (Variables|Default|SetbOverlapLeft false))

(event OnComponentBeginOverlap(Right)
  (params (OverlappedComponent :type Primitive%20Component%20Object%20Reference) (OtherActor :type Actor%20Object%20Reference) (OtherComp :type Primitive%20Component%20Object%20Reference) (OtherBodyIndex :type Integer) (bFromSweep :type Boolean) (SweepResult :type Hit%20Result%20Structure%20%28by%20ref%29))
  (Variables|Default|SetbOverlap true)
  (Variables|Default|SetbOverlapRight true))

(event OnComponentEndOverlap(Right)
  (params (OverlappedComponent :type Primitive%20Component%20Object%20Reference) (OtherActor :type Actor%20Object%20Reference) (OtherComp :type Primitive%20Component%20Object%20Reference) (OtherBodyIndex :type Integer))
  (Variables|Default|SetbOverlap false)
  (Variables|Default|SetbOverlapRight false))

(event EventBeginPlay
  (Physics|SetEnableGravity (Variables|Default|GetUp) true))

(event Collision|EventActorBeginOverlap
  (params (OtherActor :type Actor%20Object%20Reference)))

(event EventTick
  (params (DeltaSeconds :type Float%20%28single-precision%29))
  (bind _returnvalue (Game|GetPlayerController 0))
  (bind _hitresult (Game|Player|GetHitResultUnderCursorbyChannel _returnvalue "TraceTypeQuery1" true))
  (bind _location (Collision|BreakHitResult _hitresult))
  (bind (_x _y) (Math|Vector|BreakVector _location))
  ;[1 1 1] 마우스로 컴포넌트 이동
  (if (Variables|Default|GetbOnCusor)
    (switch int 0
      (:0
        (Transformation|SetWorldLocationAndRotation (Variables|Default|GetStaticMesh) (Math|Vector|MakeVector _x _y 1e+02) "0, 0, 0" false false)))))

(fn ConstructionScript)