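; BP_EnemyActor_Dragon is a dragon enemy actor with a health bar widget and a death animation.
; Any actor overlap subtracts a fixed amount from Hp and pushes it to the MonsterWidget progress bar, with no check on what overlapped.
; When Hp falls to a near-zero threshold, the mesh plays the mountain dragon death animation once and disables its collision; the actor is not destroyed.
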(event EventBeginPlay)

(event Collision|EventActorBeginOverlap
  (params (OtherActor :type Actor%20Object%20Reference))
  (bind _asmonster_widget (Utilities|Casting|CastToMonsterWidget (UserInterface|GetUserWidgetObject (Variables|Default|GetHPBarWidget))))
  (bind _output_get (Variables|Default|Sethp (- (Variables|Default|Gethp) 0.2)))
  (Progress|SetPercent (Variables|/Script/ReadiedBullet.MonsterWidget|GetHPProgressBar _asmonster_widget) _output_get)
  (if (<= (Variables|Default|Gethp) 0.1)
    (Components|Animation|PlayAnimation (Variables|Character|GetMesh) "/Game/QuadrapedCreatures/MountainDragon/Animations/ANIM_MOUNTAIN_DRAGON_death.ANIM_MOUNTAIN_DRAGON_death" false)
    (Collision|SetCollisionEnabled (Variables|Character|GetMesh) "NoCollision")))

(event EventTick
  (params (DeltaSeconds :type Float%20%28single-precision%29)))

(fn ConstructionScript)