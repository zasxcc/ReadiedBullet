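; Customization camera Blueprint that rotates its Srpin component in fixed 90-degree steps from keyboard input.
; W and S turn it in opposite directions on one axis, and A and D on another, using instant world-space rotation.
; BeginPlay shows the mouse cursor and zeroes CamRot, which the key handlers do not use.
; Tick, overlap and the construction script are empty.
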(event EventBeginPlay
  (Variables|/Script/Engine.PlayerController|SetbShowMouseCursor (Game|GetPlayerController 0) true)
  (Variables|Default|SetCamRot "0, 0, 0"))

(event Collision|EventActorBeginOverlap
  (params (OtherActor :type Actor%20Object%20Reference)))

(event EventTick
  (params (DeltaSeconds :type Float%20%28single-precision%29)))

(event Input|KeyboardEvents|A
  (params (Key :type Key%20Structure :default "None"))
  (:Pressed
    (Transformation|AddWorldRotation (Variables|Default|GetSrpin) "0.000000, 0,-90.000000" false false)))

(event Input|KeyboardEvents|D
  (params (Key :type Key%20Structure :default "None"))
  (:Pressed
    (Transformation|AddWorldRotation (Variables|Default|GetSrpin) "0.000000, 0,90.000000" false false)))

(event Input|KeyboardEvents|W
  (params (Key :type Key%20Structure :default "None"))
  (:Pressed
    (Transformation|AddWorldRotation (Variables|Default|GetSrpin) "-90.000000, 0,0.000000" false false)))

(event Input|KeyboardEvents|S
  (params (Key :type Key%20Structure :default "None"))
  (:Pressed
    (Transformation|AddWorldRotation (Variables|Default|GetSrpin) "90.000000, 0,0.000000" false false)))

(fn ConstructionScript)